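; Single-shell shotgun weapon Blueprint with flipbook animations that reloads automatically after each shot.
; ShootWeapon spends the loaded shell, calls FireShotGun, waits out the shoot animation, then triggers Reload, which refills from reserve ammo.
; DoOnce gates and a CanShoot flag block overlapping actions during animation-length delays.
; Ammo counts are read from the Player in UpdateMuns and written back on firing and reloading.
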(event Custom|resetShoot
  (bind _weaponflipbook (Variables|Default|GetWeaponFlipbook))
  (Utilities|FlowControl|DoOnce false) ; enters at Reset
)

(event Custom|ResetReload
  (bind _weaponflipbook (Variables|Default|GetWeaponFlipbook))
  (bind _player (Variables|Default|GetPlayer))
  (Utilities|FlowControl|DoOnce false) ; enters at Reset
)

(event EventBeginPlay
  (|CallParentFunction) ; This node is disabled and will not be called.\nDrag off pins to build functionality.
)

(event Collision|EventActorBeginOverlap
  (params (OtherActor :type Actor%20Object%20Reference))
  (|CallParentFunction OtherActor) ; This node is disabled and will not be called.\nDrag off pins to build functionality.
)

(event EventReload
  (bind _weaponflipbook (Variables|Default|GetWeaponFlipbook))
  (bind _player (Variables|Default|GetPlayer))
  (if (Variables|Default|GetcanShoot)
    (Utilities|FlowControl|DoOnce false
      (:Completed
        (Variables|Default|SetcanShoot false)
        (if (>= (Variables|Default|Getmunitions) (- 1.0 (Variables|Default|GetmunInGun)))
          (Audio|PlaySound2D "/Game/Sounds/Reload_Shotgun.Reload_Shotgun" 1.0 1.0 0.0 0 0)
          (Variables|Default|Setmunitions (- (Variables|Default|Getmunitions) (- 1.0 (Variables|Default|GetmunInGun))))
          (Variables|Default|SetmunInGun 1.0)
          (Variables|/Game/FirstPerson/Blueprints/BP_FirstPersonCharacter.BP_FirstPersonCharacter_C|SetShotgunMun _player (Variables|Default|GetmunInGun))
          (Variables|/Game/FirstPerson/Blueprints/BP_FirstPersonCharacter.BP_FirstPersonCharacter_C|SetMaxShotGunMun _player (Variables|Default|Getmunitions))
          (Sprite|SetFlipbook _weaponflipbook "/Game/Sprites/Weapons/ShotGun/FB_ShotGunReload.FB_ShotGunReload")
          (Utilities|FlowControl|Delay (Class|PaperFlipbookComponent|GetFlipbookLength _weaponflipbook))
          (Variables|Default|SetcanShoot true)
          (Sprite|SetFlipbook (Variables|Default|GetWeaponFlipbook) "/Game/Sprites/Weapons/ShotGun/FB_ShotGunIdle.FB_ShotGunIdle")
          (CallFunction|ResetReload))))
    (else
      (CallFunction|ResetReload))))

(event EventTick
  (params (DeltaSeconds :type Float%20%28single-precision%29))
  (|CallParentFunction DeltaSeconds) ; This node is disabled and will not be called.\nDrag off pins to build functionality.
)

(event EventUpdateMuns
  (bind _player (Variables|Default|GetPlayer))
  (Variables|Default|Setmunitions (Variables|/Game/FirstPerson/Blueprints/BP_FirstPersonCharacter.BP_FirstPersonCharacter_C|GetMaxShotGunMun _player))
  (Variables|Default|SetmunInGun (Variables|/Game/FirstPerson/Blueprints/BP_FirstPersonCharacter.BP_FirstPersonCharacter_C|GetShotgunMun _player)))

(event EventShootWeapon
  (bind _weaponflipbook (Variables|Default|GetWeaponFlipbook))
  (Utilities|FlowControl|DoOnce false
    (:Completed
      (if (Variables|Default|GetcanShoot)
        (Variables|Default|SetcanShoot false)
        (if (> (Variables|Default|GetmunInGun) 0.0)
          (Audio|PlaySound2D "/Game/Sounds/Shotgun_Shot.Shotgun_Shot" 1.0 1.0 0.0 0 0)
          (Variables|Default|SetmunInGun (- (Variables|Default|GetmunInGun) 1.0))
          (Variables|/Game/FirstPerson/Blueprints/BP_FirstPersonCharacter.BP_FirstPersonCharacter_C|SetShotgunMun (Variables|Default|GetPlayer) (Variables|Default|GetmunInGun))
          (Sprite|SetFlipbook _weaponflipbook "/Game/Sprites/Weapons/ShotGun/FB_ShotGunShoot.FB_ShotGunShoot")
          (CallFunction|FireShotGun)
          (Utilities|FlowControl|Delay (Class|PaperFlipbookComponent|GetFlipbookLength _weaponflipbook))
          (Sprite|SetFlipbook (Variables|Default|GetWeaponFlipbook) "/Game/Sprites/Weapons/ShotGun/FB_ShotGunIdle.FB_ShotGunIdle")
          (Variables|Default|SetcanShoot true)
          (CallFunction|Reload)
          (CallFunction|ResetShoot)
          (else
            (CallFunction|ResetShoot :!label _label)))
        (else
          (goto _label))))))

(fn ConstructionScript
  (|CallParentFunction))