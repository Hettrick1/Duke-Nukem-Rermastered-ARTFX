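; Base weapon Blueprint that caches the first-person player character on BeginPlay and provides hitscan firing functions.
; Fireweapon line-traces forward from the Linetrace component, ignoring itself and the player, then prints and applies WeaponDamages to the hit actor.
; FireShotGun repeats this for ten pellets, randomly offsetting each trace end point for spread.
; Shoot, stop, reload and ammo-update events are empty stubs, with no calls to either firing function here.
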(event Custom|ShootWeapon)

(event Custom|UpdateMuns)

(event Custom|Reload)

(event Custom|StopShooting)

(event EventBeginPlay
  (bind _asbp_first_person_character (Utilities|Casting|CastToBP_FirstPersonCharacter (Game|GetPlayerCharacter 0)))
  (Variables|Default|SetPlayer _asbp_first_person_character))

(event Collision|EventActorBeginOverlap
  (params (OtherActor :type Actor%20Object%20Reference)))

(event EventTick
  (params (DeltaSeconds :type Float%20%28single-precision%29)))

(fn ConstructionScript)

(fn Fireweapon
  (bind _linetrace (Variables|Default|Getlinetrace))
  (bind _weapondamages (Variables|Default|GetweaponDamages))
  (bind _returnvalue (Transformation|GetWorldLocation _linetrace))
  (bind (_outhit _returnvalue_2) (Collision|LineTraceForObjects _returnvalue (+ _returnvalue (* (Math|Vector|GetForwardVector (Transformation|GetWorldRotation (Variables|Default|Getlinetrace))) (Variables|Default|GetlinetraceDistance))) (Utilities|Array|MakeArray "ObjectTypeQuery1" "ObjectTypeQuery2" "ObjectTypeQuery3") false (Utilities|Array|MakeArray self (Game|GetPlayerCharacter 0)) "None"))
  (if _returnvalue_2
    (Development|PrintString (Utilities|String|ToString(Float) _weapondamages))
    (Game|Damage|ApplyDamage (.HitActor (Collision|BreakHitResult _outhit)) _weapondamages 0 0)))

(fn FireShotGun
  (bind _linetrace (Variables|Default|Getlinetrace))
  (bind _linetrace_2 (Variables|Default|Getlinetrace))
  (bind _linetracedistance (Variables|Default|GetlinetraceDistance))
  (bind _weapondamages (Variables|Default|GetweaponDamages))
  (bind _returnvalue (Transformation|GetWorldLocation _linetrace))
  (bind _returnvalue_2 (Transformation|GetWorldRotation _linetrace_2))
  (bind _returnvalue_3 (Math|Vector|GetForwardVector _returnvalue_2))
  (bind _returnvalue_4 (* _returnvalue_3 _linetracedistance))
  (bind _returnvalue_5 (+ _returnvalue _returnvalue_4))
  (for _index (range 1 10)
    (bind (_outhit _returnvalue_6) (Collision|LineTraceForObjects _returnvalue (Math|Vector|MakeVector (+ (.x _returnvalue_5) (Math|Random|RandomFloatinRange -1e+03 1e+03)) (+ (.y _returnvalue_5) (Math|Random|RandomFloatinRange -1e+03 1e+03)) (+ (.z _returnvalue_5) (Math|Random|RandomFloatinRange -1e+03 1e+03))) (Utilities|Array|MakeArray "ObjectTypeQuery1" "ObjectTypeQuery2" "ObjectTypeQuery3") false (Utilities|Array|MakeArray self (Game|GetPlayerCharacter 0)) "None"))
    (if _returnvalue_6
      (Development|PrintString (Utilities|String|ToString(Float) _weapondamages))
      (Game|Damage|ApplyDamage (.HitActor (Collision|BreakHitResult _outhit)) _weapondamages 0 0))))