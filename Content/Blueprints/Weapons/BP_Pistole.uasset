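; Pistol weapon Blueprint that handles shooting and reloading with Paper2D flipbook animations and syncs ammo with the Player.
; UpdateMuns pulls ammo from Player, while shots and reloads write it back.
; DoOnce gates and CanShoot block overlapping actions until each flipbook-length delay ends.
; Reload only refills a full magazine; with insufficient reserve, CanShoot and the reload gate stay locked.
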(event Custom|ResetWeapon
  (bind _weaponflipbook (Variables|Default|GetWeaponFlipbook))
  (Utilities|FlowControl|DoOnce false) ; enters at Reset
)

(event Custom|ResetReloaad
  (bind _weaponflipbook (Variables|Default|GetWeaponFlipbook))
  (bind _player (Variables|Default|GetPlayer))
  (Utilities|FlowControl|DoOnce false) ; enters at Reset
)

(event EventUpdateMuns
  (bind _player (Variables|Default|GetPlayer))
  (Variables|Default|Setmunitions (Variables|/Game/FirstPerson/Blueprints/BP_FirstPersonCharacter.BP_FirstPersonCharacter_C|GetMaxPistolMun _player))
  (Variables|Default|SetmunInGun (Variables|/Game/FirstPerson/Blueprints/BP_FirstPersonCharacter.BP_FirstPersonCharacter_C|GetPistolMun _player)))

(event Collision|EventActorBeginOverlap
  (params (OtherActor :type Actor%20Object%20Reference))
  (|CallParentFunction OtherActor))

(event EventTick
  (params (DeltaSeconds :type Float%20%28single-precision%29))
  (|CallParentFunction DeltaSeconds) ; This node is disabled and will not be called.\nDrag off pins to build functionality.
)

(event EventShootWeapon
  (bind _weaponflipbook (Variables|Default|GetWeaponFlipbook))
  (Utilities|FlowControl|DoOnce false
    (:Completed
      (if (Variables|Default|GetcanShoot)
        (if (> (Variables|Default|GetmunInGun) 0.0)
          (Variables|Default|SetmunInGun (- (Variables|Default|GetmunInGun) 1.0))
          (Variables|/Game/FirstPerson/Blueprints/BP_FirstPersonCharacter.BP_FirstPersonCharacter_C|SetPistolMun (Variables|Default|GetPlayer) (Variables|Default|GetmunInGun))
          (Variables|Default|SetcanShoot false)
          (CallFunction|Fireweapon)
          (Sprite|SetFlipbook _weaponflipbook "/Game/Sprites/Weapons/Pistol/FB_pistolShoot.FB_pistolShoot")
          (Utilities|FlowControl|Delay (Class|PaperFlipbookComponent|GetFlipbookLength _weaponflipbook))
          (Sprite|SetFlipbook (Variables|Default|GetWeaponFlipbook) "/Game/Sprites/Weapons/Pistol/FB_pistolIdle.FB_pistolIdle")
          (Variables|Default|SetcanShoot true)
          (CallFunction|ResetWeapon)
          (else
            (CallFunction|ResetWeapon :!label _label)))
        (else
          (goto _label))))))

(event EventReload
  (bind _weaponflipbook (Variables|Default|GetWeaponFlipbook))
  (bind _player (Variables|Default|GetPlayer))
  (if (Variables|Default|GetcanShoot)
    (Utilities|FlowControl|DoOnce false
      (:Completed
        (Variables|Default|SetcanShoot false)
        (if (>= (Variables|Default|Getmunitions) (- 2e+01 (Variables|Default|GetmunInGun)))
          (Variables|Default|Setmunitions (- (Variables|Default|Getmunitions) (- 2e+01 (Variables|Default|GetmunInGun))))
          (Variables|Default|SetmunInGun 2e+01)
          (Variables|/Game/FirstPerson/Blueprints/BP_FirstPersonCharacter.BP_FirstPersonCharacter_C|SetPistolMun _player (Variables|Default|GetmunInGun))
          (Variables|/Game/FirstPerson/Blueprints/BP_FirstPersonCharacter.BP_FirstPersonCharacter_C|SetMaxPistolMun _player (Variables|Default|Getmunitions))
          (Sprite|SetFlipbook _weaponflipbook "/Game/Sprites/Weapons/Pistol/FB_ReloadGun.FB_ReloadGun")
          (Utilities|FlowControl|Delay (Class|PaperFlipbookComponent|GetFlipbookLength _weaponflipbook))
          (Variables|Default|SetcanShoot true)
          (Sprite|SetFlipbook (Variables|Default|GetWeaponFlipbook) "/Game/Sprites/Weapons/Pistol/FB_pistolIdle.FB_pistolIdle")
          (CallFunction|ResetReloaad))))
    (else
      (CallFunction|ResetReloaad))))

(fn ConstructionScript
  (|CallParentFunction))