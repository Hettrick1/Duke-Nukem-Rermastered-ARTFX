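; BattleLord_BP is a sprite-based enemy that fires a machine gun at the player when it sees them.
; PawnSensing triggers a once-gated shoot flipbook, while a short delay leads to an attack sound and a forward line trace with random spread that damages BP_FirstPersonCharacter.
; A longer delay clears CanSeePlayer and resets the animation gate; when Dead, sighting the player only resets that gate instead of attacking.
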(event OnSeePawn(PawnSensing)
  (params (Pawn :type Pawn%20Object%20Reference))
  (bind _paperflipbook (Variables|Default|GetPaperFlipbook))
  (bind _scene (Variables|Default|GetScene))
  (bind _returnvalue (Transformation|GetWorldLocation _scene))
  (bind _returnvalue_2 (Transformation|GetWorldRotation _scene))
  (bind _returnvalue_3 (Math|Vector|GetForwardVector _returnvalue_2))
  (bind _returnvalue_4 (* _returnvalue_3 4e+03))
  (bind _returnvalue_5 (+ _returnvalue _returnvalue_4))
  (Utilities|FlowControl|Sequence
    (:then_0
      (Utilities|Casting|CastToBP_FirstPersonCharacter Pawn)
      (Variables|Default|SetcanSeePlayer true)
      (if (Variables|Default|Getdead)
        (CallFunction|ResetShootEnemy)
        (else
          (Utilities|FlowControl|Sequence
            (:then_0
              (Utilities|FlowControl|DoOnce false
                (:Completed
                  (Sprite|SetFlipbook _paperflipbook "/Game/Enemy/BattleLord/FB_BattleLordShoot.FB_BattleLordShoot")
                  (Utilities|FlowControl|Delay (Class|PaperFlipbookComponent|GetFlipbookLength _paperflipbook))
                  (Sprite|SetFlipbook (Variables|Default|GetPaperFlipbook) "/Game/Enemy/BattleLord/FB_BattleLordShootPosition.FB_BattleLordShootPosition"))))
            (:then_1
              (Utilities|FlowControl|Delay 0.2)
              (Audio|PlaySound2D "/Game/Sounds/Monster_Attack_machine_gun.Monster_Attack_machine_gun" 1.0 1.0 0.0 0 0)
              (bind _outhit (Collision|LineTraceForObjects _returnvalue (Math|Vector|MakeVector (+ (.x _returnvalue_5) (Math|Random|RandomFloatinRange -5e+02 5e+02)) (+ (.y _returnvalue_5) (Math|Random|RandomFloatinRange -2.5e+02 2.5e+02)) (+ (.z _returnvalue_5) (Math|Random|RandomFloatinRange -5e+02 5e+02))) (Utilities|Array|MakeArray "ObjectTypeQuery3" "ObjectTypeQuery1") false 0 "None"))
              (bind _asbp_first_person_character (Utilities|Casting|CastToBP_FirstPersonCharacter (.HitActor (Collision|BreakHitResult _outhit))))
              (Default|LoseLife _asbp_first_person_character 1e+01))))))
    (:then_1
      (Utilities|FlowControl|Delay 2.0)
      (Variables|Default|SetcanSeePlayer false)
      (CallFunction|ResetShootEnemy))))

(event Custom|ResetShootEnemy
  (bind _paperflipbook (Variables|Default|GetPaperFlipbook))
  (Utilities|FlowControl|DoOnce false) ; enters at Reset
)

(event EventBeginPlay)

(event Collision|EventActorBeginOverlap
  (params (OtherActor :type Actor%20Object%20Reference)))

(event EventTick
  (params (DeltaSeconds :type Float%20%28single-precision%29))
  (|CallParentFunction DeltaSeconds) ; This node is disabled and will not be called.\nDrag off pins to build functionality.
)

(fn ConstructionScript
  (|CallParentFunction))