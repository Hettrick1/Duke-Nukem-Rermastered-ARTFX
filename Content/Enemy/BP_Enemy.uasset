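; BP_Enemy is a flipbook-sprite enemy that chases the first-person player and dies from a single hit.
; PawnSensing sets CanSeePlayer, which is never cleared, and starts an AI move to the player, while Tick turns the enemy's yaw toward them.
; The first damage of any amount deactivates movement, plays the death flipbook, swaps to a corpse flipbook, then destroys the actor after a short delay.
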(event OnSeePawn(PawnSensing)
  (params (Pawn :type Pawn%20Object%20Reference))
  (bind _asbp_first_person_character (Utilities|Casting|CastToBP_FirstPersonCharacter Pawn))
  (Variables|Default|SetcanSeePlayer true)
  (AI|AIMoveTo self "0, 0, 0" _asbp_first_person_character 5.0 false))

(event EventBeginPlay)

(event Collision|EventActorBeginOverlap
  (params (OtherActor :type Actor%20Object%20Reference)))

(event EventTick
  (params (DeltaSeconds :type Float%20%28single-precision%29))
  (if (Variables|Default|GetcanSeePlayer)
    (Transformation|SetActorRotation (Math|Rotator|MakeRotator 0.0 0.0 (.yaw (Math|Rotator|FindLookatRotation (Transformation|GetActorLocation) (Transformation|GetActorLocation (Game|GetPlayerCharacter 0))))))))

(event Game|Damage|EventAnyDamage
  (params (Damage :type Float%20%28single-precision%29) (DamageType :type Damage%20Type%20Object%20Reference) (InstigatedBy :type Controller%20Object%20Reference) (DamageCauser :type Actor%20Object%20Reference))
  (bind _paperflipbook (Variables|Default|GetPaperFlipbook))
  (Utilities|FlowControl|DoOnce false
    (:Completed
      (Components|Activation|Deactivate (Variables|Character|GetCharacterMovement))
      (Sprite|SetFlipbook _paperflipbook "/Game/Enemy/MeleeEnemy/Death/FB_meleeDeath.FB_meleeDeath")
      (Utilities|FlowControl|Delay (Class|PaperFlipbookComponent|GetFlipbookLength _paperflipbook))
      (Sprite|SetFlipbook (Variables|Default|GetPaperFlipbook) "/Game/Enemy/MeleeEnemy/Death/FB_deadBody.FB_deadBody")
      (Utilities|FlowControl|Delay 2.0)
      (Actor|DestroyActor))))

(fn ConstructionScript)