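; Base enemy Blueprint that shows a Paper2D sprite with Doom-style directional views and handles damage and death.
; Each tick, dot products of its forward and right vectors against the player direction select the flipbook's rotation and, while idle, its directional frame.
; When it sees the player or is dead, it turns to face them.
; Damage plays a throttled hurt sound; lethal damage stops movement, plays death flipbooks, then destroys the actor.
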(event Custom|PlaySound
  (if (Variables|Default|GetcanPlaySound)
    (Variables|Default|SetcanPlaySound false)
    (Audio|PlaySound2D "/Game/Sounds/Monster_Damages.Monster_Damages" 1.0 1.0 0.0 0 0)
    (Utilities|FlowControl|Delay 0.1)
    (Variables|Default|SetcanPlaySound true)))

(event EventTick
  (params (DeltaSeconds :type Float%20%28single-precision%29))
  (bind _returnvalue (Game|GetPlayerCharacter 0))
  (bind _returnvalue_2 (Transformation|GetActorLocation))
  (bind _returnvalue_3 (Transformation|GetActorLocation _returnvalue))
  (bind _returnvalue_4 (- _returnvalue_3 _returnvalue_2))
  (bind _returnvalue_5 (Math|Vector|Normalize _returnvalue_4))
  ;[1 1 1] 8 views system
  (if (or (Variables|Default|GetcanSeePlayer) (Variables|Default|Getdead))
    (Transformation|SetActorRotation (Math|Rotator|MakeRotator 0.0 0.0 (.yaw (Math|Rotator|FindLookatRotation (Transformation|GetActorLocation) (Transformation|GetActorLocation (Game|GetPlayerCharacter 0)))))))
  (Variables|Default|Setdegrees (Class|KismetMathLibrary|DegAcos (Math|Vector|DotProduct (Transformation|GetActorForwardVector) _returnvalue_5)))
  (if (< (Math|Vector|DotProduct (Transformation|GetActorRightVector) _returnvalue_5) 0.0)
    (Math|Float|CompareFloat (Variables|Default|Getdegrees) 1.8e+02
      (:>
        (Transformation|SetRelativeRotation (Variables|Default|GetPaperFlipbook) "0.000000,-90.000000,0.000000" false false :!label _label)
        (if (not (or (Variables|Default|GetcanSeePlayer) (Variables|Default|Getdead)))
          (Sprite|SetFlipbook (Variables|Default|GetPaperFlipbook) (Utilities|Array|Get(acopy) (Variables|Default|GetflipbooksIdle)))))
      (:==
        (goto _label))
      (:<
        (Math|Float|CompareFloat (Variables|Default|Getdegrees) 135.0
          (:>
            (Transformation|SetRelativeRotation (Variables|Default|GetPaperFlipbook) "0.000000,135.000000,0.000000" false false :!label _label_2)
            (if (not (or (Variables|Default|GetcanSeePlayer) (Variables|Default|Getdead)))
              (Sprite|SetFlipbook (Variables|Default|GetPaperFlipbook) (Utilities|Array|Get(acopy) (Variables|Default|GetflipbooksIdle) 3))))
          (:==
            (goto _label_2))
          (:<
            (Math|Float|CompareFloat (Variables|Default|Getdegrees) 9e+01
              (:>
                (Transformation|SetRelativeRotation (Variables|Default|GetPaperFlipbook) "0.000000,180.000000,0.000000" false false :!label _label_3)
                (if (not (or (Variables|Default|GetcanSeePlayer) (Variables|Default|Getdead)))
                  (Sprite|SetFlipbook (Variables|Default|GetPaperFlipbook) (Utilities|Array|Get(acopy) (Variables|Default|GetflipbooksIdle) 2))))
              (:==
                (goto _label_3))
              (:<
                (Math|Float|CompareFloat (Variables|Default|Getdegrees) 45.0
                  (:>
                    _)
                  (:==
                    _)
                  (:<
                    (goto _label)))
                (Transformation|SetRelativeRotation (Variables|Default|GetPaperFlipbook) "0.000000,45.000000,0.000000" false false)
                (if (not (or (Variables|Default|GetcanSeePlayer) (Variables|Default|Getdead)))
                  (Sprite|SetFlipbook (Variables|Default|GetPaperFlipbook) (Utilities|Array|Get(acopy) (Variables|Default|GetflipbooksIdle) 1)))))))))
    (else
      (Math|Float|CompareFloat (Variables|Default|Getdegrees) 1.8e+02
        (:>
          (Transformation|SetRelativeRotation (Variables|Default|GetPaperFlipbook) "0.000000,-45.000000,0.000000" false false :!label _label_4)
          (if (not (or (Variables|Default|GetcanSeePlayer) (Variables|Default|Getdead)))
            (Sprite|SetFlipbook (Variables|Default|GetPaperFlipbook) (Utilities|Array|Get(acopy) (Variables|Default|GetflipbooksIdle) 7))))
        (:==
          (goto _label_4))
        (:<
          (Math|Float|CompareFloat (Variables|Default|Getdegrees) 135.0
            (:>
              (Transformation|SetRelativeRotation (Variables|Default|GetPaperFlipbook) "0.000000,90.000000,0.000000" false false :!label _label_5)
              (if (not (or (Variables|Default|GetcanSeePlayer) (Variables|Default|Getdead)))
                (Sprite|SetFlipbook (Variables|Default|GetPaperFlipbook) (Utilities|Array|Get(acopy) (Variables|Default|GetflipbooksIdle) 4))))
            (:==
              (goto _label_5))
            (:<
              (Math|Float|CompareFloat (Variables|Default|Getdegrees) 9e+01
                (:>
                  (Transformation|SetRelativeRotation (Variables|Default|GetPaperFlipbook) "0.000000,45.000000,0.000000" false false :!label _label_6)
                  (if (not (or (Variables|Default|GetcanSeePlayer) (Variables|Default|Getdead)))
                    (Sprite|SetFlipbook (Variables|Default|GetPaperFlipbook) (Utilities|Array|Get(acopy) (Variables|Default|GetflipbooksIdle) 5))))
                (:==
                  (goto _label_6))
                (:<
                  (Math|Float|CompareFloat (Variables|Default|Getdegrees) 45.0
                    (:>
                      _)
                    (:==
                      _))
                  (Transformation|SetRelativeRotation (Variables|Default|GetPaperFlipbook) "0, 0, 0" false false)
                  (if (not (or (Variables|Default|GetcanSeePlayer) (Variables|Default|Getdead)))
                    (Sprite|SetFlipbook (Variables|Default|GetPaperFlipbook) (Utilities|Array|Get(acopy) (Variables|Default|GetflipbooksIdle) 6))))))))))))

(event Game|Damage|EventAnyDamage
  (params (Damage :type Float%20%28single-precision%29) (DamageType :type Damage%20Type%20Object%20Reference) (InstigatedBy :type Controller%20Object%20Reference) (DamageCauser :type Actor%20Object%20Reference))
  (bind _paperflipbook (Variables|Default|GetPaperFlipbook))
  (if (> (Variables|Default|GetenemyLife) Damage)
    (Variables|Default|SetenemyLife (- (Variables|Default|GetenemyLife) Damage))
    (CallFunction|PLaySOund)
    (else
      (Variables|Default|SetenemyLife 0.0)
      (Utilities|FlowControl|DoOnce false
        (:Completed
          (Variables|Default|Setdead true)
          (Components|Activation|Deactivate (Variables|Character|GetCharacterMovement))
          (Sprite|SetFlipbook _paperflipbook (Variables|Default|GetdeadFB))
          (Audio|PlaySound2D "/Game/Sounds/Monster_Die.Monster_Die" 1.0 1.0 0.0 0 0)
          (Utilities|FlowControl|Delay (Class|PaperFlipbookComponent|GetFlipbookLength _paperflipbook))
          (Sprite|SetFlipbook (Variables|Default|GetPaperFlipbook) (Variables|Default|GetdeadBodyFB))
          (Utilities|FlowControl|Delay 2.0)
          (Actor|DestroyActor))))))

(fn ConstructionScript)